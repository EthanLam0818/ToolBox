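; BP_ItemAmount_World is an actor that shows a list of item amounts through a WBP_ItemGridPanel in its Widget component.
; It initializes the panel in the construction script and again on BeginPlay, passing the item list, a horizontal/vertical layout setting and a show-maximum setting.
; Every Tick it casts the widget and pushes the current item amount list to the panel, so the display refreshes by polling.
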(event `self.ReceiveBeginPlay`
  (`self.初始化panel`))

(event `self.ReceiveTick`
  (params (DeltaSeconds :type "Float (single-precision)"))
  (bind _aswbp_item_grid_panel (cast `/Game/工具箱/控件/UserWidget/WBP_ItemGridPanel` (`WidgetComponent.GetWidget` (`self.Widget`))))
  (`/Game/工具箱/控件/UserWidget/WBP_ItemGridPanel.更新amount` _aswbp_item_grid_panel (`self.物品数量list`)))

(fn `UserConstructionScript`
  (`self.初始化panel`))

(fn `初始化panel`
  (bind _aswbp_item_grid_panel (cast `/Game/工具箱/控件/UserWidget/WBP_ItemGridPanel` (`WidgetComponent.GetWidget` (`self.Widget`))))
  (`/Game/工具箱/控件/UserWidget/WBP_ItemGridPanel.初始化` _aswbp_item_grid_panel (`self.横 / 竖`) (`self.显示最大值`) (`self.物品数量list`)))
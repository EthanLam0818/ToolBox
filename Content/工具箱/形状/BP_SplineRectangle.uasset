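; Construction-script shape tool that builds a rectangle spline with rounded corners from Size and Radius.
; A helper Spline holds four sharp corners scaled from a unit square, and BuildSplineOnRadius turns each edge into two points on a newly added MainSpline.
; Radius is clamped to half the edge length, and tangents of twice that inset along each edge curve the corners.
; Optional flags then build spline meshes or fill the shape, each followed by ArrowDir.
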(fn `BuildSplineOnRadius`
  (bind _mainspline (`self.MainSpline`))
  (bind _spline (`self.Spline`))
  (for _index (range (`SplineComponent.GetNumberOfSplinePoints` (`self.Spline`)))
    (bind _returnvalue (`SplineComponent.GetLocationAtSplinePoint` _spline (+ _index 1) "Local"))
    (bind _returnvalue_2 (`SplineComponent.GetLocationAtSplinePoint` _spline _index "Local"))
    (bind _returnvalue_3 (`KismetMathLibrary.FClamp` (`self.Radius`) 0.0 (/ (`KismetMathLibrary.Vector_Distance` _returnvalue_2 _returnvalue) 2.0)))
    (bind _returnvalue_4 (* (`KismetMathLibrary.Normal` (- _returnvalue _returnvalue_2)) _returnvalue_3))
    (bind _returnvalue_5 (* _index 2))
    (`SplineComponent.AddSplinePointAtIndex` _mainspline (+ _returnvalue_4 _returnvalue_2) _returnvalue_5 "Local" true)
    (bind _returnvalue_6 (* _returnvalue_4 (`KismetMathLibrary.Conv_DoubleToVector` 2.0)))
    (`SplineComponent.SetTangentsAtSplinePoint` _mainspline _returnvalue_5 _returnvalue_6 (0.0 0.0 0.0) "Local" true)
    (bind _returnvalue_7 (+ (* _index 2) 1))
    (`SplineComponent.AddSplinePointAtIndex` _mainspline (+ _returnvalue (* (`KismetMathLibrary.Normal` (- _returnvalue_2 _returnvalue)) _returnvalue_3)) _returnvalue_7 "Local" true)
    (`SplineComponent.SetTangentsAtSplinePoint` _mainspline _returnvalue_7 (0.0 0.0 0.0) _returnvalue_6 "Local" true)))

(fn `UserConstructionScript`
  (bind _spline (`self.Spline`))
  (bind `_样条线网格_build` (break `/Game/工具箱/形状/Other/S_SplineMesh` (`self.样条线网格`)))
  (bind (`_填充形状_fill` `_填充形状_fillmat` `_填充形状_fillcolor`) (break `/Game/工具箱/形状/Other/S_FillShape` (`self.填充形状`)))
  (set `self.Alpha?Radius` false)
  (`SplineComponent.ClearSplinePoints` (`self.Spline`) true)
  (for (_array_element _array_index) (`|MakeArray` (-0.5 -0.5 0.0) (-0.5 0.5 0.0) (0.5 0.5 0.0) (0.5 -0.5 0.0) :!type "Vector Structure")
    (`SplineComponent.AddSplinePointAtIndex` _spline (* _array_element (`self.size`)) _array_index "Local" true)
    (`SplineComponent.SetTangentAtSplinePoint` _spline _array_index (0.0 0.0 0.0) "Local" true))
  (bind _returnvalue (`AddComponent|NODE_AddSplineComponent-0`))
  (bind _output_get (set `self.MainSpline` _returnvalue))
  (`SplineComponent.ClearSplinePoints` _output_get true)
  (`self.BuildSplineOnRadius`)
  (`|ExecutionSequence`
    (:`then_0`
      (if `_样条线网格_build`
        (`self.BuildSplineMesh`)
        (`self.ArrowDir` :!label _label)))
    (:`then_1`
      (if `_填充形状_fill`
        (`self.FillShape` `_填充形状_fillmat` `_填充形状_fillcolor`)
        (goto _label)))))
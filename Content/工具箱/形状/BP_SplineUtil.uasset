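; Spline utility actor that turns an editable linear control spline into a generated spline with rounded corners.
; The construction script straightens the control points, then builds MainSpline by inserting tangent points around each corner, placed by lerp Alpha or clamped Radius.
; Optionally, it tiles spline meshes along the result and orients an arrow at the start.
; FillShape builds a tinted procedural triangle-fan mesh from sampled spline points; Tick can draw point indices for debugging.
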(event `self.ReceiveTick`
  (params (DeltaSeconds :type "Float (single-precision)"))
  (bind _mainspline (`self.MainSpline`))
  (if (`self.DebugPointIndex`)
    (for _index (range (+ (`SplineComponent.GetNumberOfSplinePoints` _mainspline) 1))
      (`KismetSystemLibrary.DrawDebugString` (+ (`SplineComponent.GetLocationAtSplinePoint` _mainspline _index "World") (0.0 0.0 0.0)) (`KismetStringLibrary.Conv_IntToString` _index) null (struct :`G` 5.0 :`A` 1.0)))))

(fn `ArrowDir`
  (bind _mainspline (`self.MainSpline`))
  (`SceneComponent.K2_SetWorldTransform` (`self.Arrow`) (`KismetMathLibrary.MakeTransform` (`SplineComponent.GetLocationAtSplinePoint` _mainspline 0 "World") (`SplineComponent.GetRotationAtSplinePoint` _mainspline 0 "World")) false false))

(fn `BuildSplineMesh`
  (bind _mainspline (`self.MainSpline`))
  (bind (`_样条线网格_build` `_样条线网格_mesh` `_样条线网格_meshaxis` `_样条线网格_meshlenght`) (break `/Game/工具箱/形状/Other/S_SplineMesh` (`self.样条线网格`)))
  (bind (`_样条线网格_build_2` `_样条线网格_mesh_2` `_样条线网格_meshaxis_2` `_样条线网格_meshlenght_2` `_样条线网格_meshscale` `_样条线网格_meshmaterial`) (break `/Game/工具箱/形状/Other/S_SplineMesh` (`self.样条线网格`)))
  (bind (_x _y) (`KismetMathLibrary.BreakVector2D` `_样条线网格_meshscale`))
  (for _index (range (+ (`KismetMathLibrary.FFloor` (/ (`SplineComponent.GetSplineLength` (`self.MainSpline`)) `_样条线网格_meshlenght`)) 1))
    (bind _returnvalue (`AddComponent|NODE_AddSplineMeshComponent-0`))
    (`SplineMeshComponent.SetForwardAxis` _returnvalue `_样条线网格_meshaxis_2` true)
    (`StaticMeshComponent.SetStaticMesh` _returnvalue `_样条线网格_mesh_2`)
    (`PrimitiveComponent.SetMaterial` _returnvalue 0 `_样条线网格_meshmaterial`)
    (bind _returnvalue_2 (* `_样条线网格_meshlenght` _index))
    (bind _returnvalue_3 (* (+ _index 1) `_样条线网格_meshlenght`))
    (`SplineMeshComponent.SetStartAndEnd` _returnvalue (`SplineComponent.GetLocationAtDistanceAlongSpline` _mainspline _returnvalue_2 "Local") (`SplineComponent.GetDirectionAtDistanceAlongSpline` _mainspline _returnvalue_2 "Local") (`SplineComponent.GetLocationAtDistanceAlongSpline` _mainspline _returnvalue_3 "Local") (`SplineComponent.GetDirectionAtDistanceAlongSpline` _mainspline _returnvalue_3 "Local") true)
    (`SplineMeshComponent.SetStartScale` _returnvalue (`KismetMathLibrary.MakeVector2D` _x _y) true)
    (`SplineMeshComponent.SetEndScale` _returnvalue (`KismetMathLibrary.MakeVector2D` _x _y) true)))

(fn `BuildSplineOnLerp`
  (bind _spline (`self.Spline`))
  (bind _mainspline (`self.MainSpline`))
  (bind _mainspline_2 (`self.MainSpline`))
  (bind _spline_2 (`self.Spline`))
  (bind _spline_3 (`self.Spline`))
  (bind _alpha (`self.Alpha`))
  (bind _returnvalue (`SplineComponent.GetNumberOfSplinePoints` (`self.Spline`)))
  (bind _returnvalue_2 (- _returnvalue 1))
  (for _index (range (+ _returnvalue_2 1))
    (`/Engine/EditorBlueprintResources/StandardMacros.CompareFloat` (`self.Alpha`) 0.5
      (:`>`
        (if (!= _index _returnvalue_2) :!label _label
          (bind _returnvalue_3 (`SplineComponent.GetLocationAtSplinePoint` _spline_2 _index "Local"))
          (bind _returnvalue_4 (`SplineComponent.GetLocationAtSplinePoint` _spline_2 (+ _index 1) "Local"))
          (bind _returnvalue_5 (`KismetMathLibrary.VLerp` _returnvalue_3 _returnvalue_4 _alpha))
          (bind _returnvalue_6 (+ _index 1))
          (`SplineComponent.AddSplinePointAtIndex` _mainspline _returnvalue_5 _returnvalue_6 "Local" true)
          (`SplineComponent.SetTangentAtSplinePoint` _mainspline _returnvalue_6 (* (`KismetMathLibrary.Vector_Distance` _returnvalue_3 _returnvalue_4) (`KismetMathLibrary.Normal` (- _returnvalue_4 _returnvalue_3))) "Local" true)
          (else
            (`SplineComponent.AddSplinePointAtIndex` _mainspline (`SplineComponent.GetLocationAtSplinePoint` _spline (- (`SplineComponent.GetNumberOfSplinePoints` _spline) 1) "Local") _returnvalue_6 "Local" true)
            (`SplineComponent.SetTangentAtSplinePoint` _mainspline _returnvalue_6 (0.0 0.0 0.0) "Local" true))))
      (:`==`
        (goto _label))
      (:`<`
        (bind _returnvalue_7 (+ (* _index 2) 1))
        (`SplineComponent.AddSplinePointAtIndex` _mainspline_2 _returnvalue_5 _returnvalue_7 "Local" true)
        (bind _returnvalue_8 (* (`KismetMathLibrary.Normal` (- _returnvalue_5 _returnvalue_3)) (* (`KismetMathLibrary.Vector_Distance` _returnvalue_5 _returnvalue_3) 2.0)))
        (`SplineComponent.SetTangentAtSplinePoint` _mainspline_2 _returnvalue_7 _returnvalue_8 "Local" true)
        (if (!= _index (- _returnvalue 2))
          (bind _returnvalue_9 (+ (* _index 2) 2))
          (`SplineComponent.AddSplinePointAtIndex` _mainspline_2 (`KismetMathLibrary.VLerp` _returnvalue_3 _returnvalue_4 (- 1.0 _alpha)) _returnvalue_9 "Local" true)
          (`SplineComponent.SetTangentAtSplinePoint` _mainspline_2 _returnvalue_9 _returnvalue_8 "Local" true)
          (else
            (`SplineComponent.AddSplinePointAtIndex` _mainspline_2 (`SplineComponent.GetLocationAtSplinePoint` _spline_3 (- (`SplineComponent.GetNumberOfSplinePoints` _spline_3) 1) "Local") _returnvalue_9 "Local" true)
            (`SplineComponent.SetTangentAtSplinePoint` _mainspline_2 _returnvalue_9 (0.0 0.0 0.0) "Local" true)))))))

(fn `BuildSplineOnRadius`
  (bind _mainspline (`self.MainSpline`))
  (bind _spline (`self.Spline`))
  (bind (`_样条线网格_build` `_样条线网格_mesh` `_样条线网格_meshaxis` `_样条线网格_meshlenght`) (break `/Game/工具箱/形状/Other/S_SplineMesh` (`self.样条线网格`)))
  (bind _spline_2 (`self.Spline`))
  (bind _returnvalue (- (`SplineComponent.GetNumberOfSplinePoints` (`self.Spline`)) 2))
  (for _index (range (+ _returnvalue 1))
    (bind _returnvalue_2 (`SplineComponent.GetLocationAtSplinePoint` _spline (+ _index 1) "Local"))
    (bind _returnvalue_3 (`SplineComponent.GetLocationAtSplinePoint` _spline _index "Local"))
    (bind _returnvalue_4 (/ (`KismetMathLibrary.Vector_Distance` _returnvalue_3 _returnvalue_2) 2.0))
    (bind _returnvalue_5 (`KismetMathLibrary.FMin` (`KismetMathLibrary.SelectFloat` (- _returnvalue_4 `_样条线网格_meshlenght`) _returnvalue_4 `_样条线网格_build`) (`self.Radius`)))
    (bind _returnvalue_6 (* (`KismetMathLibrary.Normal` (- _returnvalue_2 _returnvalue_3)) _returnvalue_5))
    (bind _returnvalue_7 (+ (* _index 2) 1))
    (`SplineComponent.AddSplinePointAtIndex` _mainspline (+ _returnvalue_6 _returnvalue_3) _returnvalue_7 "Local" true)
    (bind _returnvalue_8 (* _returnvalue_6 (`KismetMathLibrary.Conv_DoubleToVector` 2.0)))
    (`SplineComponent.SetTangentsAtSplinePoint` _mainspline _returnvalue_7 _returnvalue_8 (`KismetMathLibrary.MakeVector` 0.0) "Local" true)
    (if (!= _index _returnvalue)
      (bind _returnvalue_9 (+ (* _index 2) 2))
      (`SplineComponent.AddSplinePointAtIndex` _mainspline (+ _returnvalue_2 (* (`KismetMathLibrary.Normal` (- _returnvalue_3 _returnvalue_2)) _returnvalue_5)) _returnvalue_9 "Local" true)
      (`SplineComponent.SetTangentsAtSplinePoint` _mainspline _returnvalue_9 (`KismetMathLibrary.MakeVector` 0.0) _returnvalue_8 "Local" true)
      (else
        (`SplineComponent.AddSplinePointAtIndex` _mainspline (`SplineComponent.GetLocationAtSplinePoint` _spline_2 (- (`SplineComponent.GetNumberOfSplinePoints` _spline_2) 1) "Local") _returnvalue_9 "Local" true)
        (`SplineComponent.SetTangentAtSplinePoint` _mainspline _returnvalue_9 (0.0 0.0 0.0) "Local" true)))))

(fn `FillShape`
  (params (Material :type "MaterialInterface Object Reference") (Color :type "LinearColor Structure"))
  (locals (point :type "Array of Vector Structure") (Index :type "Array of Integer"))
  (bind (_r _g _b _a) (`KismetMathLibrary.BreakColor` Color))
  (bind _index (`local.Index`))
  (bind _mainspline (`self.MainSpline`))
  (bind _sample (`self.sample`))
  (bind _returnvalue (`AddComponent|NODE_AddProceduralMeshComponent-0`))
  (bind _output_get (set `self.ProMesh` _returnvalue))
  (`PrimitiveComponent.SetMaterial` _output_get 0 Material)
  (`|ExecutionSequence`
    (:`then_0`
      (`KismetArrayLibrary.Array_Clear` (`local.point`))
      (`KismetArrayLibrary.Array_Set` (`local.point`) 0 (0.0 0.0 0.0) true)
      (for _index_2 (range (+ (`SplineComponent.GetNumberOfSplinePoints` _mainspline) 1))
        (for _index_3 (range (+ _sample 1))
          (`KismetArrayLibrary.Array_Add` (`local.point`) (`SplineComponent.GetLocationAtDistanceAlongSpline` _mainspline (`KismetMathLibrary.Lerp` (`SplineComponent.GetDistanceAlongSplineAtSplinePoint` _mainspline _index_2) (`SplineComponent.GetDistanceAlongSplineAtSplinePoint` _mainspline (+ _index_2 1)) (/ (`KismetMathLibrary.Conv_IntToDouble` _index_3) (`KismetMathLibrary.Conv_IntToDouble` _sample))) "Local"))))
      (for _index_4 (range (+ (- (`KismetArrayLibrary.Array_Length` (`local.point`)) 3) 1))
        (`KismetArrayLibrary.Array_Set` _index (* _index_4 3) 0 true)
        (`KismetArrayLibrary.Array_Set` _index (+ (* _index_4 3) 1) (+ _index_4 1) true)
        (`KismetArrayLibrary.Array_Set` _index (+ (* _index_4 3) 2) (+ _index_4 2) true))
      (`ProceduralMeshComponent.CreateMeshSection_LinearColor` :`self` (`self.ProMesh`) :`Vertices` (`local.point`) :`Triangles` (`local.Index`)))
    (:`then_1`
      (`MeshComponent.SetVectorParameterValueOnMaterials` _output_get "颜色叠加" (`KismetMathLibrary.MakeVector` _r _g _b))
      (`MeshComponent.SetScalarParameterValueOnMaterials` _output_get "Opacity_Max" _a))))

(fn `UserConstructionScript`
  (bind `_样条线网格_build` (break `/Game/工具箱/形状/Other/S_SplineMesh` (`self.样条线网格`)))
  (bind _spline (`self.Spline`))
  (for _index (range (+ (`SplineComponent.GetNumberOfSplinePoints` _spline) 1))
    (`SplineComponent.SetSplinePointType` _spline _index "Linear" true))
  (bind _returnvalue (`AddComponent|NODE_AddSplineComponent-0`))
  (bind _output_get (set `self.MainSpline` _returnvalue))
  (`SplineComponent.ClearSplinePoints` _output_get true)
  (`SplineComponent.AddSplinePointAtIndex` (`self.MainSpline`) (`SplineComponent.GetLocationAtSplinePoint` (`self.Spline`) 0 "Local") 0 "Local" true)
  (if (`self.Alpha?Radius`)
    (`self.BuildSplineOnLerp`)
    (else
      (`self.BuildSplineOnRadius`)))
  (if `_样条线网格_build`
    (`self.BuildSplineMesh`)
    (`self.ArrowDir`)))
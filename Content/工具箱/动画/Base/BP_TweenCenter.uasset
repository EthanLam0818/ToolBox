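; BP_TweenCenter is a central manager actor that drives registered tween animations.
; AddTween and RemoveTween maintain a duplicate-free list, which a fast looping timer started on BeginPlay processes instead of Tick.
; PlayUpdate turns game time since each tween's start into normalized progress, inverted for reversed tweens, and passes it to OnPlayUpdate.
; Once progress exceeds the end, it calls OnPlayEnd without removing the tween itself.
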(event `self.ReceiveBeginPlay`
  (`KismetSystemLibrary.K2_SetTimerDelegate` (delegate `CustomEvent_0`) 0.01 true))

(event `CustomEvent_0`
  (`/Engine/EditorBlueprintResources/StandardMacros.CompareInt` (`KismetArrayLibrary.Array_Length` (`self.TweenList`))
    (:`>`
      (`self.Play Update`))))

(fn `AddTween`
  (params (Item :type "/Game/工具箱/动画/Base/TB_CMP_TweenBase Object Reference (by ref)"))
  (bind _tweenlist (`self.TweenList`))
  (if (not (`KismetArrayLibrary.Array_Contains` _tweenlist Item))
    (`KismetArrayLibrary.Array_Add` _tweenlist Item)))

(fn `Play Update`
  (locals (tempTween :type "/Game/工具箱/动画/Base/S_TweenInfo Structure"))
  (bind (_temptween_tween _temptween_starttime _temptween_durationtime _temptween_easetype _temptween_easefunc _temptween_playsetting) (break `/Game/工具箱/动画/Base/S_TweenInfo` (`local.tempTween`)))
  (bind _temptween_tween_2 (break `/Game/工具箱/动画/Base/S_TweenInfo` (`local.tempTween`)))
  (bind _returnvalue (/ (- (`KismetSystemLibrary.GetGameTimeInSeconds`) _temptween_starttime) _temptween_durationtime))
  ;[0 0.1 1] 更新计时器
  (for _array_element (`self.TweenList`)
    (set `local.tempTween` (`/Game/工具箱/动画/Base/TB_CMP_TweenBase.TweenInfo` _array_element))
    (`/Engine/EditorBlueprintResources/StandardMacros.CompareFloat` _returnvalue 1.0
      (:`>`
        (`/Game/工具箱/动画/Base/TB_CMP_TweenBase.OnPlayEnd` _temptween_tween_2))
      (:`==`
        (`/Game/工具箱/动画/Base/TB_CMP_TweenBase.OnPlayUpdate` _temptween_tween_2 (`KismetMathLibrary.SelectFloat` (- 1.0 _returnvalue) _returnvalue (`.isReverse_19_44183C754F5E164E76DFF7B4B2155FD8` (break `/Game/工具箱/动画/Base/S_PlaySetting` _temptween_playsetting))) :!label _label))
      (:`<`
        (goto _label)))))

(fn `RemoveTween`
  (params (item :type "/Game/工具箱/动画/Base/TB_CMP_TweenBase Object Reference (by ref)"))
  (bind _tweenlist (`self.TweenList`))
  (if (`KismetArrayLibrary.Array_Contains` _tweenlist item)
    (`KismetArrayLibrary.Array_RemoveItem` _tweenlist item)))

(fn `UserConstructionScript`)
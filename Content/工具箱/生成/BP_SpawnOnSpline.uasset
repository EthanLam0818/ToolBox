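; Toolbox actor that places copies of a chosen class (Spawn目标) along the MainSpline of a target spline actor.
; The construction script fills point and rotation arrays by fixed distance or by count, adding a shared rotation offset to the spline rotation.
; A one-shot 显示位置 flag draws debug boxes and direction cones at those points.
; Spawn, not called within the graphs, creates an actor at each stored transform and attaches it to this actor.
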(fn `GetPointsAtCount`
  (bind _mainspline (`/Game/工具箱/形状/TB_BP_SplineUtil.MainSpline` (`self.目标Spline`)))
  (set `self. Dinstance` (/ (`SplineComponent.GetSplineLength` _mainspline) (`KismetMathLibrary.Conv_IntToDouble` (`self.Count`))))
  (for _index (range (+ (`self.Count`) 1))
    (bind _returnvalue (* (`self. Dinstance`) _index))
    (bind _returnvalue_2 (`SplineComponent.GetLocationAtDistanceAlongSpline` _mainspline _returnvalue "World"))
    (`KismetArrayLibrary.Array_Set` (`self.points`) _index _returnvalue_2 true)
    (bind _returnvalue_3 (`KismetMathLibrary.ComposeRotators` (`SplineComponent.GetRotationAtDistanceAlongSpline` _mainspline _returnvalue "Local") (`self.统一旋转`)))
    (`KismetArrayLibrary.Array_Set` (`self.rotation`) _index _returnvalue_3 true)
    (if (`self.显示位置`)
      (`KismetSystemLibrary.DrawDebugBox` _returnvalue_2 (10.0 10.0 10.0) (struct :`R` 0.022174 :`G` 1.0 :`A` 1.0) _returnvalue_3 1.0)
      (`KismetSystemLibrary.DrawDebugConeInDegrees` (+ _returnvalue_2 (* (`KismetMathLibrary.Conv_DoubleToVector` 30.0) (`KismetMathLibrary.GetForwardVector` _returnvalue_3))) (`KismetMathLibrary.GetForwardVector` (`KismetMathLibrary.ComposeRotators` _returnvalue_3 (struct :`Yaw` 180.0))) 20.0 45.0 45.0 12 (struct :`R` 0.021898 :`G` 1.0 :`A` 1.0) 1.0)))
  (set `self.显示位置` false))

(fn `GetPointsAtDistance`
  (bind _mainspline (`/Game/工具箱/形状/TB_BP_SplineUtil.MainSpline` (`self.目标Spline`)))
  (set `self.Count` (`KismetMathLibrary.FCeil` (/ (`SplineComponent.GetSplineLength` _mainspline) (`self. Dinstance`))))
  (for _index (range (+ (`self.Count`) 1))
    (bind _returnvalue (* (`self. Dinstance`) _index))
    (bind _returnvalue_2 (`SplineComponent.GetLocationAtDistanceAlongSpline` _mainspline _returnvalue "World"))
    (`KismetArrayLibrary.Array_Set` (`self.points`) _index _returnvalue_2 true)
    (bind _returnvalue_3 (`KismetMathLibrary.ComposeRotators` (`SplineComponent.GetRotationAtDistanceAlongSpline` _mainspline _returnvalue "Local") (`self.统一旋转`)))
    (`KismetArrayLibrary.Array_Set` (`self.rotation`) _index _returnvalue_3 true)
    (if (`self.显示位置`)
      (`KismetSystemLibrary.DrawDebugBox` _returnvalue_2 (10.0 10.0 10.0) (struct :`R` 0.022174 :`G` 1.0 :`A` 1.0) _returnvalue_3 1.0)
      (`KismetSystemLibrary.DrawDebugConeInDegrees` (+ _returnvalue_2 (* (`KismetMathLibrary.Conv_DoubleToVector` 30.0) (`KismetMathLibrary.GetForwardVector` _returnvalue_3))) (`KismetMathLibrary.GetForwardVector` (`KismetMathLibrary.ComposeRotators` _returnvalue_3 (struct :`Yaw` 180.0))) 20.0 45.0 45.0 12 (struct :`R` 0.021898 :`G` 1.0 :`A` 1.0) 1.0)))
  (set `self.显示位置` false))

(fn `Spawn`
  (locals (NewLocalVar_0 :type "Actor Class Reference"))
  (for (_array_element _array_index) (`self.points`)
    (bind _returnvalue (`|SpawnActorFromClass` (`self.Spawn目标`) (`KismetMathLibrary.MakeTransform` _array_element (`|GetArrayItem` (`self.rotation`) _array_index)) "Undefined" "OverrideRootScale" null null))
    (`self.K2_AttachToActor` _returnvalue self "None" "KeepWorld" "KeepRelative" "KeepRelative" true)))

(fn `UserConstructionScript`
  (`KismetArrayLibrary.Array_Clear` (`self.points`))
  (if (`self.SpanwAt?Distance:Count`)
    (`self.GetPointsAtDistance`)
    (else
      (`self.GetPointsAtCount`))))
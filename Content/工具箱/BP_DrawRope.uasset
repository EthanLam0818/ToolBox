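; Rope actor that builds a physics-driven rope between itself and an attached end actor, previewed through the Construction Script and updated every Tick.
; Capsule colliders, counted from distance over segment height with an optional length cap, are chained by physics constraints from a Sphere to the end actor.
; A spline follows the capsule positions, and fixed-length spline mesh segments are added or destroyed along it to render the rope.
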(event `self.ReceiveBeginPlay`
  (set `self.isPlay` true))

(event `self.ReceiveTick`
  (params (DeltaSeconds :type "Float (single-precision)"))
  (`self.Update Rope Info`)
  (`self.Update Spline`)
  (`self.Update SpineMesh`))

(fn `Add Colider`
  (params (Index :type Integer) (Location :type "Vector Structure"))
  (returns (ReturnValue :type "CapsuleComponent Object Reference"))
  (bind (_returnvalue_location _returnvalue_rotation) (`KismetMathLibrary.BreakTransform` (`KismetAnimationLibrary.K2_LookAt` (`self.GetTransform`) (`self.K2_GetActorLocation` (`self.attachEndActor`)) (0.0 0.0 1.0) false (0.0 1.0 0.0))))
  (bind _returnvalue (`AddComponent|NODE_AddCapsuleComponent-0`))
  (`SceneComponent.K2_SetWorldLocationAndRotation` _returnvalue (`self.K2_GetActorLocation`) _returnvalue_rotation false false)
  (`KismetArrayLibrary.Array_Insert` (`self.colliders`) _returnvalue)
  (`CapsuleComponent.SetCapsuleHalfHeight` _returnvalue (- (/ (`self.colliderHight`) 2.0) 10.0) true)
  (`CapsuleComponent.SetCapsuleRadius` _returnvalue (`self.colliderRadius`) true)
  (return _returnvalue))

(fn `End Constraints`
  (params (collider :type "PrimitiveComponent Object Reference"))
  (`/Engine/EditorBlueprintResources/StandardMacros.IsValid` (`self.End Constraint`)
    (:`Is Valid`
      _)
    (:`Is Not Valid`
      (bind _returnvalue (`AddComponent|NODE_AddPhysicsConstraintComponent-1`))
      (set `self.End Constraint` _returnvalue)
      (`KismetArrayLibrary.Array_Insert` (`self.constraints`))))
  (`SceneComponent.K2_AttachToComponent` (`self.End Constraint`) collider "None" "KeepRelative" "KeepRelative" "KeepRelative" true)
  (`PhysicsConstraintComponent.SetConstrainedComponents` (`self.End Constraint`) collider "None" (`self.GetComponentByClass` (`self.attachEndActor`) "/Script/Engine.PrimitiveComponent") "None"))

(fn `GetLocation`
  (params (currIndext :type "Float (double-precision)"))
  (returns (LerpPosition :type "Vector Structure"))
  (return (`KismetMathLibrary.VLerp` (`self.K2_GetActorLocation`) (`self.K2_GetActorLocation` (`self.attachEndActor`)) (- 1.0 (/ currIndext (`KismetMathLibrary.Conv_IntToDouble` (`self.colliderCount`)))))))

(fn `Update Rope Info`
  (locals (currIndex :type Integer) (currCollider :type "CapsuleComponent Object Reference"))
  (bind _colliders (`self.colliders`))
  (bind _currindex (`local.currIndex`))
  (bind _colliders_2 (`self.colliders`))
  (bind _output (`|GetArrayItem` (`self.constraints`) (`local.currIndex`)))
  (if (`self.first`)
    (for _array_element _colliders
      (`/Engine/EditorBlueprintResources/StandardMacros.IsValid` _array_element
        (:`Is Valid`
          (`ActorComponent.K2_DestroyComponent` _array_element))))
    (`KismetArrayLibrary.Array_Clear` _colliders)
    (set `self.first` false))
  (`self.UpdateCountCamp`)
  (for _index (range (+ (`self.colliderCount`) 1))
    (bind _output_get (set `local.currIndex` _index))
    (`/Engine/EditorBlueprintResources/StandardMacros.CompareInt` _output_get (`KismetArrayLibrary.Array_Length` _colliders_2)
      (:`>`
        (bind _returnvalue (`self.Add Colider` (`local.currIndex`) (`self.GetLocation` (`KismetMathLibrary.Conv_IntToDouble` (`local.currIndex`))) :!label _label))
        (set `local.currCollider` _returnvalue)
        (bind _returnvalue_2 (`AddComponent|NODE_AddPhysicsConstraintComponent-0` :!label _label_2))
        (`SceneComponent.K2_AttachToComponent` _returnvalue_2 (`local.currCollider`) "None" "KeepRelative" "KeepRelative" "KeepRelative" true)
        (`KismetArrayLibrary.Array_Set` (`self.constraints`) (`local.currIndex`) _returnvalue_2 true))
      (:`==`
        (bind _output_2 (`|GetArrayItem` _colliders_2 _output_get))
        (`/Engine/EditorBlueprintResources/StandardMacros.IsValid` _output_2 :!label _label_3
          (:`Is Valid`
            (if (not (`self.isPlay`))
              (`SceneComponent.K2_SetWorldLocation` _output_2 (`self.GetLocation` (`KismetMathLibrary.Conv_IntToDouble` (`local.currIndex`))) false false))
            (bind _output_get_2 (set `local.currCollider` _output_2))
            (if (== (`local.currIndex`) 0)
              (`self.End Constraints` _output_get_2))
            (`/Engine/EditorBlueprintResources/StandardMacros.IsValid` (`|GetArrayItem` (`self.constraints`) (`local.currIndex`))
              (:`Is Valid`
                _)
              (:`Is Not Valid`
                (goto _label_2))))
          (:`Is Not Valid`
            (goto _label))))
      (:`<`
        (goto _label_3)))
    (`PhysicsConstraintComponent.SetConstrainedComponents` _output (select `bool` (== _currindex 0) :`false` (`|GetArrayItem` (`self.colliders`) (- _currindex 1)) :`true` (`self.Sphere`) :!type "PrimitiveComponent Object Reference") "None" (`local.currCollider`) "None")
    (if (!= 0 (`local.currIndex`))
      (`PhysicsConstraintComponent.SetConstraintReferencePosition` _output "Frame1" (`KismetMathLibrary.MakeVector` 0.0 0.0 (`self.colliderHight`)))
      (else
        (`PhysicsConstraintComponent.SetConstraintReferencePosition` _output "Frame1" (0.0 0.0 0.0))))
    (`PhysicsConstraintComponent.SetConstraintReferencePosition` _output "Frame2" (0.0 0.0 0.0))
    (if (== _currindex (`self.colliderCount`))
      _)))

(fn `Update SpineMesh`
  (locals (NewLocalVar_0 :type Integer :default 0))
  (bind _meshlenght (`self.meshLenght`))
  (bind _spline (`self.Spline`))
  (bind _meshscale (`self.meshScale`))
  (bind _returnvalue (`SplineComponent.GetSplineLength` (`self.Spline`)))
  (bind _output_get (set `local.NewLocalVar_0` (`KismetMathLibrary.FFloor` (/ _returnvalue _meshlenght))))
  (for _index (range (+ _output_get 1))
    (bind _output (`|GetArrayItem` (`self.splineMeshs`) _index))
    (`/Engine/EditorBlueprintResources/StandardMacros.IsValid` _output
      (:`Is Valid`
        _)
      (:`Is Not Valid`
        (bind _returnvalue_2 (`AddComponent|NODE_AddSplineMeshComponent-0`))
        (`KismetArrayLibrary.Array_Set` (`self.splineMeshs`) _index _returnvalue_2 true)))
    (`SplineMeshComponent.SetStartScale` _output (`KismetMathLibrary.MakeVector2D` _meshscale _meshscale) true)
    (`SplineMeshComponent.SetEndScale` _output (`KismetMathLibrary.MakeVector2D` _meshscale _meshscale) true)
    (bind _returnvalue_3 (* _index _meshlenght))
    (bind _returnvalue_4 (`KismetMathLibrary.SelectFloat` _returnvalue (* (+ _index 1) _meshlenght) (== _index (`local.NewLocalVar_0`))))
    (`SplineMeshComponent.SetStartAndEnd` _output (`SplineComponent.GetLocationAtDistanceAlongSpline` _spline _returnvalue_3 "Local") (`SplineComponent.GetTangentAtDistanceAlongSpline` _spline _returnvalue_3 "Local") (`SplineComponent.GetLocationAtDistanceAlongSpline` _spline _returnvalue_4 "Local") (`SplineComponent.GetTangentAtDistanceAlongSpline` _spline _returnvalue_4 "Local") true)
    (`SplineMeshComponent.SetStartRoll` _output 0.0 true)
    (`SplineMeshComponent.SetEndRoll` _output 0.0 true))
  (for (_array_element _array_index) (`self.splineMeshs`)
    (if (> _array_index (`local.NewLocalVar_0`))
      (`/Engine/EditorBlueprintResources/StandardMacros.IsValid` _array_element
        (:`Is Valid`
          (`ActorComponent.K2_DestroyComponent` _array_element))))))

(fn `Update Spline`
  (for (_array_element _array_index) (`self.colliders`)
    (`KismetArrayLibrary.Array_Set` (`self.points`) _array_index (`SceneComponent.K2_GetComponentLocation` _array_element) true))
  (`SplineComponent.SetSplinePoints` (`self.Spline`) (`self.points`) "World" true))

(fn `UpdateCountCamp`
  (bind _maxcount (`self.maxCount`))
  (bind _returnvalue (`KismetMathLibrary.FFloor` (/ (`KismetMathLibrary.Vector_Distance` (`self.K2_GetActorLocation`) (`self.K2_GetActorLocation` (`self.attachEndActor`))) (`self.colliderHight`))))
  (set `self.maxCount` (`KismetMathLibrary.FFloor` (/ (`self.maxLenght`) (`self.colliderHight`))))
  (if (== 0 (`self.maxCount`))
    (set `self.colliderCount` _returnvalue)
    (elif (< _maxcount _returnvalue)
      (set `self.colliderCount` _maxcount)
      (else
        (set `self.colliderCount` _returnvalue)))))

(fn `UserConstructionScript`
  (`KismetArrayLibrary.Array_Clear` (`self.colliders`))
  (if (`self.attachEnd`)
    (`/Engine/EditorBlueprintResources/StandardMacros.IsValid` (`self.attachEndActor`)
      (:`Is Valid`
        (`self.Update Rope Info`)
        ;[0 0 1] Draw Rope
        (`self.Update Spline`)
        (`self.Update SpineMesh`))
      (:`Is Not Valid`
        (`KismetSystemLibrary.PrintString` "没有附加末端")))))
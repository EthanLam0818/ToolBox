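; TB_CMP_Rotate is a tween component that rotates its owning actor from a starting rotation to a target rotation.
; InitTween stores the target, duration, loop and ping-pong settings, then calls Begin to start the tween.
; TweenUpdate calls the parent update, then sets the actor's rotation by lerping from the start transform's rotation to the target, using a float curve sampled at Timer as alpha.
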(fn `InitTween`
  (params (Target :type "Rotator Structure") (`持续时间` :type "Float (double-precision)") (`Is Loop` :type Boolean) (isPingPong :type Boolean))
  (set `self.Target` Target)
  (set `self.持续时间` `持续时间`)
  (set `self.Is Loop` `Is Loop`)
  (set `self.isPingPong` isPingPong)
  (`self.Begin`))

(fn `TweenUpdate`
  (bind (`_起始变换_location` `_起始变换_rotation`) (`KismetMathLibrary.BreakTransform` (`self.起始变换`)))
  (`parent.TweenUpdate`)
  (`Actor.K2_SetActorRotation` (`self.GetOwner`) (`KismetMathLibrary.RLerp` `_起始变换_rotation` (`self.Target`) (`CurveFloat.GetFloatValue` (`self.曲线`) (`self.timer`))) false))
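; Tween component that moves its owning actor to a target location, part of an animation toolbox.
; InitTween stores the target, duration, loop and ping-pong settings, then calls Begin; its Reverse and NewParam inputs are unused.
; The TweenUpdate override runs the parent update, then sets the actor location by lerping from the start transform to the target with Timer as alpha, without sweep.
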(fn `InitTween`
  (params (`目标` :type "Vector Structure" :default (0.0 0.0 0.0)) (`持续时间` :type "Float (double-precision)" :default 0.0) (`循环` :type Boolean :default false) (isPingPong :type Boolean :default false) (Reverse :type Boolean) (NewParam :type Boolean))
  (set `self.Target` `目标`)
  (set `self.持续时间` `持续时间`)
  (set `self.Is Loop` `循环`)
  (set `self.isPingPong` isPingPong)
  (`self.Begin`))

(fn `TweenUpdate`
  (bind `_起始变换_location` (`KismetMathLibrary.BreakTransform` (`self.起始变换`)))
  (`parent.TweenUpdate`)
  (`Actor.K2_SetActorLocation` (`self.GetOwner`) (`KismetMathLibrary.VLerp` `_起始变换_location` (`self.Target`) (`self.timer`)) false false))
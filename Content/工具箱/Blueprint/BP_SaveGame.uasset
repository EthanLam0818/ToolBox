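; SaveGame object for the ToolBox tool that stores a history of target materials in a name-keyed map.
; MatHistoryADD removes the first key when the map holds more than five entries, then removes and re-adds the given name to refresh it.
; Save writes the object itself to the "ToolBox" slot and prints the result; adding to history does not trigger it.
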(fn `MatHistory_ADD`
  (params (Name :type "String (by ref)") (Value :type "MaterialInstanceConstant Object Reference (by ref)"))
  (bind _targetmathistory (`self.targetMatHistory`))
  (bind _returnvalue (`BlueprintMapLibrary.Map_Length` _targetmathistory))
  (`/Engine/EditorBlueprintResources/StandardMacros.CompareInt` _returnvalue 5
    (:`>`
      (bind _keys (`BlueprintMapLibrary.Map_Keys` _targetmathistory))
      (for _ (range (+ (- _returnvalue 6) 1))
        (`BlueprintMapLibrary.Map_Remove` _targetmathistory (`|GetArrayItem` _keys))))
    (:`==`
      _)
    (:`<`
      _))
  (if (`BlueprintMapLibrary.Map_Contains` _targetmathistory Name)
    (bind _returnvalue_2 (`BlueprintMapLibrary.Map_Remove` _targetmathistory Name))
    (if _returnvalue_2
      (`BlueprintMapLibrary.Map_Add` (`self.targetMatHistory`) Name Value :!label _label))
    (else
      (goto _label))))

(fn `Save`
  (bind _returnvalue (`GameplayStatics.SaveGameToSlot` self "ToolBox"))
  (`KismetSystemLibrary.PrintString` null (`KismetStringLibrary.Concat_StrStr` "【ToolBox】SaveGame修改保存---" (`KismetStringLibrary.Conv_BoolToString` _returnvalue))))
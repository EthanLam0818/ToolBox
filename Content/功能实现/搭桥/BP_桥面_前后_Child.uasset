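; Child Blueprint of a bridge deck piece (桥面, front/back variant) for the bridge-building feature, inheriting its runtime behavior from the parent.
; It overrides the binding initialization (初始化绑定), calling the parent and then registering the four corner anchors as keep-size components.
; It also sets the length-adjustment list for the road surface, right-side anchors and a physics constraint, each with scale, offset and mode settings.
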(fn `UserConstructionScript`
  (`parent.UserConstructionScript`))

(fn `初始化绑定`
  (`parent.初始化绑定`)
  (set `self.保持大小的锚点` (`|MakeArray` (`self.左前锚`) (`self.左后锚`) :!type "SceneComponent Object Reference"))
  (set `self.长度调整_对象` (`|MakeArray` (make `/Game/功能实现/搭桥/Blueprint/Struct/S长度调整` (`self.路面`) (0.5 0.5 0.5) 0.0 0.0 "NewEnumerator1") (make `/Game/功能实现/搭桥/Blueprint/Struct/S长度调整` (`self.右后锚`) (1.0 1.0 1.0) -39.0 1.0) (make `/Game/功能实现/搭桥/Blueprint/Struct/S长度调整` (`self.右前锚`) (1.0 1.0 1.0) 39.0 1.0) :!type "/Game/功能实现/搭桥/Blueprint/Struct/S长度调整 Structure"))
  (`KismetArrayLibrary.Array_Append` (`self.保持大小的锚点`) (`|MakeArray` (`self.右前锚`) (`self.右后锚`) :!type "SceneComponent Object Reference"))
  (`KismetArrayLibrary.Array_Add` (`self.长度调整_对象`) (make `/Game/功能实现/搭桥/Blueprint/Struct/S长度调整` (`self.PhysicsConstraint1`) (1.0 1.0 1.0) 0.0 1.0 "NewEnumerator1")))
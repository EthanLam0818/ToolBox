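; Base bridge-member actor for a bridge-building feature, stretched between its own anchor and a target actor, with physics simulation switched on by a trigger event.
; It rolls its root toward the target in the YZ plane, repositioning and scaling listed components to span the distance while resizing selected anchors.
; A physics constraint binds it to another bridge piece or an anchor's mesh.
; Tick prints a debug "Hello"; velocity-based colouring is unconnected.
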(event `self.ReceiveBeginPlay`
  (for _array_element (`SceneComponent.GetChildrenComponents` (`self.root`) false)
    (bind `_as静态网格体组件` (cast `StaticMeshComponent` _array_element))
    (`PrimitiveComponent.SetCollisionEnabled` `_as静态网格体组件` "NoCollision")
    (`self.更新约束`)))

(event `Trigger模拟物理`
  (`PrimitiveComponent.SetSimulatePhysics` (`self.root`) true))

(event `self.ReceiveActorBeginOverlap`
  (params (OtherActor :type "Actor Object Reference")))

(event `self.ReceiveTick`
  (params (DeltaSeconds :type "Float (single-precision)"))
  (`self.新函数_0`)
  (if (`self.长度调整_Active`)
    (`self.自动调整长度`)
    (`self.锚点保持大小`)))

(fn `UserConstructionScript`
  (`self.初始化绑定`)
  (`self.更新约束`)
  (`self.自动调整长度`)
  (`self.锚点保持大小`))

(fn `初始化绑定`
  (set `self.网格组件list` (`self.K2_GetComponentsByClass` "/Script/Engine.MeshComponent")))

(fn `新函数_0`
  (`KismetSystemLibrary.PrintString` "Hello"))

(fn `更新约束`
  (bind _root (`self.root`))
  (bind `_约束对象_锚点` (`self.约束对象_锚点`))
  (bind _physicsconstraint (`self.PhysicsConstraint`))
  (`self.自动调整长度`)
  (`/Engine/EditorBlueprintResources/StandardMacros.IsValid` `_约束对象_锚点`
    (:`Is Valid`
      (bind `_asbp_桥梁base` (cast `/Game/功能实现/搭桥/Blueprint/LowPoly/BP_桥梁Base` `_约束对象_锚点`)
        (:`then`
          (`PhysicsConstraintComponent.SetConstrainedComponents` _physicsconstraint (`/Game/功能实现/搭桥/Blueprint/LowPoly/BP_桥梁Base.root` `_asbp_桥梁base`) "root" _root "root"))
        (:`CastFailed`
          (`PhysicsConstraintComponent.SetConstrainedComponents` _physicsconstraint (`|GetArrayItem` (`self.K2_GetComponentsByClass` `_约束对象_锚点` "/Script/Engine.StaticMeshComponent")) "root" _root "root"))))
    (:`Is Not Valid`
      (`PhysicsConstraintComponent.SetConstrainedComponents` _physicsconstraint null "None" _root "root"))))

(fn `自动调整长度`
  (bind _returnvalue_x (`KismetMathLibrary.BreakVector` (`self.K2_GetActorLocation`)))
  (bind _returnvalue (`self.K2_GetActorLocation`))
  (bind `_长度调整_目标` (`self.长度调整_目标`))
  (bind _returnvalue_2 (`self.K2_GetActorLocation` `_长度调整_目标`))
  (bind _returnvalue_3 (* (`self.锚点大小`) 2.0))
  (bind _returnvalue_4 (- _returnvalue _returnvalue_2))
  (bind _returnvalue_5 (/ (`KismetMathLibrary.VSize` _returnvalue_4) 100.0))
  (`/Engine/EditorBlueprintResources/StandardMacros.IsValid` `_长度调整_目标`
    (:`Is Valid`
      ;[0 0 1] Root会自动旋转对其到目标
      (`SceneComponent.K2_SetWorldRotation` (`self.root`) (`KismetMathLibrary.MakeRotator` (+ (* (/ (`KismetMathLibrary.Atan2` (.y _returnvalue_4) (.z _returnvalue_4)) (`KismetMathLibrary.GetPI`)) 180.0) -90.0)) false false)
      ;[0.006141 0 1] 调整长度与位置
      (for _array_element (`self.长度调整_对象`)
        (bind (`_组件` `_基础缩放` `_x位置偏移` `_伸缩轴心` `_伸缩轴向`) (break `/Game/功能实现/搭桥/Blueprint/Struct/S长度调整` _array_element))
        (`SceneComponent.K2_SetWorldLocation` `_组件` (`KismetMathLibrary.MakeVector` (+ `_x位置偏移` _returnvalue_x) (.y (- _returnvalue (* (- _returnvalue _returnvalue_2) (`KismetMathLibrary.Conv_DoubleToVector` `_伸缩轴心`)))) (.z (- _returnvalue (* (- _returnvalue _returnvalue_2) (`KismetMathLibrary.Conv_DoubleToVector` `_伸缩轴心`))))) false false)
        (switch `/Game/工具箱/Blueprint/Enum/E_XYZ` `_伸缩轴向`
          (:`NewEnumerator1`
            (bind _returnvalue_6 (* (.x `_基础缩放`) _returnvalue_3))
            (`SceneComponent.SetRelativeScale3D` `_组件` (`KismetMathLibrary.MakeVector` _returnvalue_6 _returnvalue_5 (* (.z `_基础缩放`) _returnvalue_3))))
          (:`NewEnumerator2`
            (`SceneComponent.SetRelativeScale3D` `_组件` (`KismetMathLibrary.MakeVector` _returnvalue_6 (* (.y `_基础缩放`) _returnvalue_3) _returnvalue_5))))))))

(fn `锚点保持大小`
  (locals (NewLocalVar_0 :type "Vector Structure" :default (0.06 0.1 0.1)))
  (for _array_element (`self.保持大小的锚点`)
    (`SceneComponent.SetWorldScale3D` _array_element (* (`self.锚点比例`) (`self.锚点大小`)))))
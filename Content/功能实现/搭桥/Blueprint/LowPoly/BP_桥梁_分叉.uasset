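; BP_桥梁_分叉 is a forked bridge piece for a physics-based bridge-building feature, adding a second anchor connection.
; Its 更新约束 override runs the parent logic, then binds PhysicsConstraint1 between 约束对象锚点2 and its own Root.
; Bridge and front-deck anchors attach by their "root" bone, other actors by their first static mesh component.
; With no valid anchor, only the Root side is set.
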(fn `UserConstructionScript`
  (`parent.UserConstructionScript`))

(fn `更新约束`
  (bind _root (`self.root`))
  (bind `_约束对象_锚点2` (`self.约束对象_锚点2`))
  (bind _physicsconstraint1 (`self.PhysicsConstraint1`))
  (`parent.更新约束`)
  (`/Engine/EditorBlueprintResources/StandardMacros.IsValid` `_约束对象_锚点2`
    (:`Is Valid`
      (bind `_asbp_桥梁` (cast `/Game/功能实现/搭桥/Blueprint/LowPoly/BP_桥梁` `_约束对象_锚点2`)
        (:`then`
          (`PhysicsConstraintComponent.SetConstrainedComponents` _physicsconstraint1 (`/Game/功能实现/搭桥/Blueprint/LowPoly/BP_桥梁.root` `_asbp_桥梁`) "root" _root "root"))
        (:`CastFailed`
          (bind `_asbp_桥面_前` (cast `/Game/功能实现/搭桥/Blueprint/LowPoly/BP_桥面_前` `_约束对象_锚点2`)
            (:`then`
              (`PhysicsConstraintComponent.SetConstrainedComponents` _physicsconstraint1 (`/Game/功能实现/搭桥/Blueprint/LowPoly/BP_桥面_前.root` `_asbp_桥面_前`) "root" _root "root"))
            (:`CastFailed`
              (`PhysicsConstraintComponent.SetConstrainedComponents` _physicsconstraint1 (`|GetArrayItem` (`self.K2_GetComponentsByClass` `_约束对象_锚点2` "/Script/Engine.StaticMeshComponent")) "None" _root "root"))))))
    (:`Is Not Valid`
      (`PhysicsConstraintComponent.SetConstrainedComponents` _physicsconstraint1 null "None" _root "root"))))
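; BP_桥面_前 is a low-poly front bridge-deck piece for the bridge-building feature, derived from a parent Blueprint that supplies the logic.
; It overrides 初始化绑定 (binding initialization) to register the left-front and left-rear anchors as size-preserving and the road surface (路面) as the sole length-adjusted object.
; Tick and the construction script only call the parent.
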(event `self.ReceiveBeginPlay`)

(event `self.ReceiveTick`
  (params (DeltaSeconds :type "Float (single-precision)"))
  (`parent.ReceiveTick` DeltaSeconds))

(fn `UserConstructionScript`
  (`parent.UserConstructionScript`))

(fn `初始化绑定`
  (`parent.初始化绑定`)
  (set `self.保持大小的锚点` (`|MakeArray` (`self.左前锚`) (`self.左后锚`) :!type "SceneComponent Object Reference"))
  (set `self.长度调整_对象` (`|MakeArray` (make `/Game/功能实现/搭桥/Blueprint/Struct/S长度调整` (`self.路面`) (1.0 1.0 1.0)) :!type "/Game/功能实现/搭桥/Blueprint/Struct/S长度调整 Structure")))
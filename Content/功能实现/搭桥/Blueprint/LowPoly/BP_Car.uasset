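; BP_Car is a physics-driven van for a bridge-building feature that drives forward or breaks constrained structures around it.
; A Start event sets 发动 (engine on), so Tick adds velocity along the Arrow's forward vector with slight lift, scaled by 前进推力 (thrust).
; When 坍塌 (collapse) is true, Tick instead runs a debug-drawn sphere trace at the van, breaking every physics constraint on hit actors.
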(event `Start`
  (set `self.发动` true))

(event `self.ReceiveTick`
  (params (DeltaSeconds :type "Float (single-precision)"))
  (bind _returnvalue (`SceneComponent.K2_GetComponentLocation` (`self.SK_Veh_Car_Van_01`)))
  (if (`self.坍塌`)
    (bind _outhits (`KismetSystemLibrary.SphereTraceMulti` :`Start` _returnvalue :`End` _returnvalue :`Radius` (`self.Radius`) :`TraceChannel` "TraceTypeQuery1" :`DrawDebugType` "ForDuration" :`DrawTime` 0.1))
    (for _array_element _outhits
      (bind (_bblockinghit _binitialoverlap _time _distance _location _impactpoint _normal _impactnormal _physmat _hitactor) (`GameplayStatics.BreakHitResult` _array_element))
      (`/Engine/EditorBlueprintResources/StandardMacros.IsValid` _hitactor
        (:`Is Valid`
          (for _array_element_2 (`self.K2_GetComponentsByClass` _hitactor "/Script/Engine.PhysicsConstraintComponent")
            (`PhysicsConstraintComponent.BreakConstraint` _array_element_2)))))
    (elif (`self.发动`)
      (`PrimitiveComponent.SetPhysicsLinearVelocity` (`self.SK_Veh_Car_Van_01`) (* (+ (`SceneComponent.GetForwardVector` (`self.Arrow`)) (0.0 0.0 0.2)) (`self.前进推力`)) true "None"))))

(fn `UserConstructionScript`)
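; Base Blueprint for a beam (梁) in the bridge-building (搭桥) feature, specializing a parent class that provides the binding and anchor-sizing logic.
; 初始化绑定 registers two anchors to keep their size and two components, with mirrored offsets, for length adjustment.
; 锚点保持大小 extends the parent by setting Head's world scale, applying the anchor size to Y and Z while fixing X at one.
; BeginPlay and Tick only call the parent.
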(event `self.ReceiveBeginPlay`
  (`parent.ReceiveBeginPlay`))

(event `self.ReceiveTick`
  (params (DeltaSeconds :type "Float (single-precision)"))
  (`parent.ReceiveTick` DeltaSeconds))

(fn `UserConstructionScript`
  (`parent.UserConstructionScript`))

(fn `初始化绑定`
  (`parent.初始化绑定`)
  (set `self.保持大小的锚点` (`|MakeArray` (`self.anchor1`) (`self.anchor2`) :!type "SceneComponent Object Reference"))
  (set `self.长度调整_对象` (`|MakeArray` (make `/Game/功能实现/搭桥/Blueprint/Struct/S长度调整` (`self.untitled1`) (0.05 0.05 1.0) -50.0 1.0) (make `/Game/功能实现/搭桥/Blueprint/Struct/S长度调整` (`self.untitled2`) (0.05 0.05 1.0) 50.0 1.0) :!type "/Game/功能实现/搭桥/Blueprint/Struct/S长度调整 Structure")))

(fn `锚点保持大小`
  (bind `_锚点大小` (`self.锚点大小`))
  (`parent.锚点保持大小`)
  (`SceneComponent.SetWorldScale3D` (`self.head`) (* (1.0 1.0 1.0) (`KismetMathLibrary.MakeVector` 1.0 `_锚点大小` `_锚点大小`))))
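; BP_物理管理 is the physics manager for the bridge-building feature, switching bridge pieces between simulated and reset states.
; Start模拟 finds every BP_桥梁Base actor, turns off length adjustment, updates its constraints and triggers physics simulation.
; 重置桥梁 instead gathers BP_梁_Base actors, updates constraints, re-runs automatic length adjustment and disables physics on mesh components directly under each Root.
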(event `self.ReceiveBeginPlay`)

(event `Start模拟`
  (bind _outactors (`GameplayStatics.GetAllActorsOfClass` "/Game/功能实现/搭桥/BP_桥梁Base.BP_桥梁Base_C"))
  (for _array_element _outactors
    (set `/Game/功能实现/搭桥/BP_桥梁Base.长度调整_Active` false _array_element)
    (`/Game/功能实现/搭桥/BP_桥_Base前.更新约束` _array_element)
    (`/Game/功能实现/搭桥/BP_桥_Base前.Trigger模拟物理` _array_element)))

(fn `UserConstructionScript`)

(fn `重置桥梁`
  (bind _outactors (`GameplayStatics.GetAllActorsOfClass` "/Game/功能实现/搭桥/BP_梁_Base.BP_梁_Base_C"))
  (for _array_element _outactors
    (`/Game/功能实现/搭桥/BP_梁_Base.更新约束` _array_element)
    (`/Game/功能实现/搭桥/BP_梁_Base.自动调整长度` _array_element)
    (for _array_element_2 (`SceneComponent.GetChildrenComponents` (`/Game/功能实现/搭桥/BP_桥梁Base.root` _array_element) false)
      (bind `_as网格体组件` (cast `MeshComponent` _array_element_2))
      (`PrimitiveComponent.SetSimulatePhysics` `_as网格体组件` false))))
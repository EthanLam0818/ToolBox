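; Child Blueprint for the rear bridge deck piece (桥面_后) in a bridge-building feature.
; 初始化绑定 gathers the mesh components, sets the left front and left rear anchors as size-preserving anchors, and registers the road surface (路面) for length adjustment.
; ChangeColor extends the parent by pushing the color to the road material, with alpha driving both blend and emissive strength.
; Event graph stubs are disabled and the construction script only calls the parent.
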(fn `ChangeColor`
  (params (color :type "LinearColor Structure"))
  (bind (_r _g _b _a) (`KismetMathLibrary.BreakColor` color))
  (bind `_路面` (`self.路面`))
  (`parent.ChangeColor` color)
  (`MeshComponent.SetVectorParameterValueOnMaterials` `_路面` "颜色混合" (`KismetMathLibrary.Conv_LinearColorToVector` color))
  (`MeshComponent.SetScalarParameterValueOnMaterials` `_路面` "混合强度" _a)
  (`MeshComponent.SetScalarParameterValueOnMaterials` `_路面` "Emissiove_强度" _a))

(fn `UserConstructionScript`
  (`parent.UserConstructionScript`))

(fn `初始化绑定`
  (set `self.网格组件list` (`self.K2_GetComponentsByClass` "/Script/Engine.MeshComponent"))
  (set `self.保持大小的锚点` (`|MakeArray` (`self.左前锚`) (`self.左后锚`) :!type "SceneComponent Object Reference"))
  (set `self.长度调整_对象` (`|MakeArray` (make `/Game/功能实现/搭桥/Blueprint/Struct/S长度调整` (`self.路面`) (0.5 0.5 0.5) 0.0 0.0 "NewEnumerator1") :!type "/Game/功能实现/搭桥/Blueprint/Struct/S长度调整 Structure")))
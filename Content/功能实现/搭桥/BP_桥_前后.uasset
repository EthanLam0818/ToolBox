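; Bridge-building piece (桥_前后, front/back) that extends a parent bridge Blueprint with additional anchors and a physics constraint.
; Binding setup registers both added anchors for scale keeping and the constraint for length adjustment.
; Constraint updates join the root to the second anchor's target: a front-base bridge or beam root, otherwise its first static mesh.
; Without a valid target, the constraint's second component stays empty.
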(event `self.ReceiveBeginPlay`
  (`parent.ReceiveBeginPlay`))

(fn `UserConstructionScript`
  (`parent.UserConstructionScript`))

(fn `初始化绑定`
  (`parent.初始化绑定`)
  (`KismetArrayLibrary.Array_Append` (`self.保持大小的锚点`) (`|MakeArray` (`self.sm_anchor3`) (`self.sm_anchor2`) :!type "SceneComponent Object Reference"))
  (`KismetArrayLibrary.Array_Add` (`self.长度调整_对象`) (make `/Game/功能实现/搭桥/Blueprint/Struct/S长度调整` (`self.PhysicsConstraint1`) (1.0 1.0 1.0))))

(fn `更新约束`
  (bind `_约束对象_锚点2` (`self.约束对象_锚点2`))
  (bind _physicsconstraint1 (`self.PhysicsConstraint1`))
  (bind _root (`self.root`))
  (`parent.更新约束`)
  (`/Engine/EditorBlueprintResources/StandardMacros.IsValid` `_约束对象_锚点2`
    (:`Is Valid`
      (bind `_asbp_桥_base前` (cast `/Game/功能实现/搭桥/BP_桥_Base前` `_约束对象_锚点2`)
        (:`then`
          (`PhysicsConstraintComponent.SetConstrainedComponents` _physicsconstraint1 _root "root" (`/Game/功能实现/搭桥/BP_桥_Base前.root` `_asbp_桥_base前`) "root"))
        (:`CastFailed`
          (bind `_asbp_梁_base` (cast `/Game/功能实现/搭桥/BP_梁_Base` `_约束对象_锚点2`)
            (:`then`
              (`PhysicsConstraintComponent.SetConstrainedComponents` _physicsconstraint1 _root "root" (`/Game/功能实现/搭桥/BP_桥梁Base.root` `_asbp_梁_base`) "root"))
            (:`CastFailed`
              (`PhysicsConstraintComponent.SetConstrainedComponents` _physicsconstraint1 _root "root" (`|GetArrayItem` (`self.K2_GetComponentsByClass` `_约束对象_锚点2` "/Script/Engine.StaticMeshComponent")) "None"))))))
    (:`Is Not Valid`
      (`PhysicsConstraintComponent.SetConstrainedComponents` _physicsconstraint1 _root "root" null "None"))))

(fn `锚点保持大小`
  (bind _returnvalue (* (`self.锚点比例`) (`self.锚点大小`)))
  (`parent.锚点保持大小`)
  (`SceneComponent.SetWorldScale3D` (`self.sm_anchor3`) _returnvalue)
  (`SceneComponent.SetWorldScale3D` (`self.sm_anchor2`) _returnvalue))
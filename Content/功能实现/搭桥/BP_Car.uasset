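; BP_Car is a thruster-driven car for a bridge-building feature that breaks physics constraints on actors around it.
; Its Start event activates the PhysicsThruster, waits a configurable delay, then starts a looping 0.1-second timer.
; Each tick runs a stationary multi-sphere trace on Visibility at the car's location and breaks every PhysicsConstraintComponent on the hit actors.
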(event `Start`
  (`ActorComponent.SetActive` (`self.PhysicsThruster`) true true)
  (`KismetSystemLibrary.Delay` (`self.掉落距离开始的间隔`))
  (`KismetSystemLibrary.K2_SetTimerDelegate` (delegate `自定义事件_0`) 0.1 true))

(event `自定义事件_0`
  (bind _returnvalue (`self.K2_GetActorLocation`))
  (bind _outhits (`KismetSystemLibrary.SphereTraceMulti` _returnvalue _returnvalue (`self.Radius`) "TraceTypeQuery1"))
  (for _array_element _outhits
    (bind (_bblockinghit _binitialoverlap _time _distance _location _impactpoint _normal _impactnormal _physmat _hitactor) (`GameplayStatics.BreakHitResult` _array_element))
    (`/Engine/EditorBlueprintResources/StandardMacros.IsValid` _hitactor
      (:`Is Valid`
        (for _array_element_2 (`self.K2_GetComponentsByClass` _hitactor "/Script/Engine.PhysicsConstraintComponent")
          (`PhysicsConstraintComponent.BreakConstraint` _array_element_2))))))

(fn `UserConstructionScript`)
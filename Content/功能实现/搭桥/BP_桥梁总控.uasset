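; Bridge master controller that automatically builds a bridge piece by piece, then starts a physics simulation with cars.
; When auto-build is enabled, it hides the queued pieces, then on Tick reveals each in turn, sliding it from its length-adjust target to its original position with a color-curve tint.
; After the last piece, Start模拟 resets all bridge actors, enables their physics and starts every BP_Car.
; 重置桥梁 switches bridge physics off.
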(event `self.ReceiveBeginPlay`
  (`|ExecutionSequence`
    (:`then_1`
      (if (`self.启用自动建造`)
        (for _array_element (`self.动画队列`)
          (`self.SetActorHiddenInGame` _array_element true))))))

(event `self.ReceiveTick`
  (params (DeltaSeconds :type "Float (single-precision)"))
  (if (`self.启用自动建造`)
    (`self.自动建造`)))

(fn `Start模拟`
  (bind _outactors (`GameplayStatics.GetAllActorsOfClass` "/Game/功能实现/搭桥/Blueprint/LowPoly/BP_桥梁Base.BP_桥梁Base_C"))
  (for _array_element _outactors
    (`/Game/功能实现/搭桥/Blueprint/LowPoly/BP_桥梁Base.Reset` _array_element)
    (set `/Game/功能实现/搭桥/Blueprint/LowPoly/BP_桥梁Base.长度调整_Active` false _array_element)
    (`PrimitiveComponent.SetSimulatePhysics` (`/Game/功能实现/搭桥/Blueprint/LowPoly/BP_桥梁Base.root` _array_element) true)
    (`KismetSystemLibrary.PrintString` (`KismetSystemLibrary.GetDisplayName` _array_element)))
  (bind _outactors_2 (`GameplayStatics.GetAllActorsOfClass` "/Game/功能实现/搭桥/Blueprint/LowPoly/BP_Car.BP_Car_C"))
  (for _array_element_2 _outactors_2
    (`/Game/功能实现/搭桥/Blueprint/LowPoly/BP_Car.Start` _array_element_2)))

(fn `UserConstructionScript`)

(fn `自动建造`
  (locals (NewLocalVar_0 :type "Actor Object Reference"))
  (bind `_动画index` (`self.动画Index`))
  (bind _output (`|GetArrayItem` (`self.动画队列`) `_动画index`))
  (bind _returnvalue (- (`KismetSystemLibrary.GetGameTimeInSeconds`) (`self.currTimer`)))
  (bind _returnvalue_2 (/ _returnvalue (`self.生长时间`)))
  (`/Engine/EditorBlueprintResources/StandardMacros.CompareInt` `_动画index` (`KismetArrayLibrary.Array_Length` (`self.动画队列`))
    (:`==`
      (if (not (`self.开始模拟`))
        (set `self.开始模拟` true)
        (`self.Start模拟`)))
    (:`<`
      (if (`self.正在播放`)
        (`self.SetActorHiddenInGame` _output false)
        (`/Engine/EditorBlueprintResources/StandardMacros.CompareFloat` _returnvalue (+ (`self.生长时间`) (`self.停顿时间`))
          (:`>`
            (`/Game/功能实现/搭桥/Blueprint/LowPoly/BP_桥梁Base.ChangeColor` :`self` _output)
            (bind _result (`/Engine/EditorBlueprintResources/StandardMacros.IncrementInt` (`self.动画Index`))
              (:`  `
                (`/Engine/EditorBlueprintResources/StandardMacros.CompareInt` _result (`KismetArrayLibrary.Array_Length` (`self.动画队列`))
                  (:`<`
                    (set `self.正在播放` false))))))
          (:`==`
            (`/Engine/EditorBlueprintResources/StandardMacros.IsValid` _output :!label _label
              (:`Is Valid`
                (`self.K2_SetActorLocation` _output (`KismetMathLibrary.VLerp` (`self.K2_GetActorLocation` (`/Game/功能实现/搭桥/Blueprint/LowPoly/BP_桥梁Base.长度调整_目标` _output)) (`self.form`) (`KismetMathLibrary.FClamp` _returnvalue_2)) false false)
                (`/Game/功能实现/搭桥/Blueprint/LowPoly/BP_桥梁Base.ChangeColor` _output (`CurveLinearColor.GetLinearColorValue` (`self.color`) _returnvalue_2)))))
          (:`<`
            (goto _label)))
        (else
          (set `self.form` (`self.K2_GetActorLocation` _output))
          (set `self.currTimer` (`KismetSystemLibrary.GetGameTimeInSeconds`))
          (set `self.正在播放` true))))))

(fn `重置桥梁`
  (bind _outactors (`GameplayStatics.GetAllActorsOfClass` "/Game/功能实现/搭桥/Blueprint/LowPoly/BP_桥梁Base.BP_桥梁Base_C"))
  (for _array_element _outactors
    (`PrimitiveComponent.SetSimulatePhysics` (`/Game/功能实现/搭桥/Blueprint/LowPoly/BP_桥梁Base.root` _array_element) false)))
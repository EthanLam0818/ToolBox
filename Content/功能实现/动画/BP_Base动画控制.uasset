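; Base Blueprint for procedural animation of actors and components, with an empty 动画执行 function left for children to define the motion.
; An optional delayed looping timer advances 曲线时间, driving 控制队列 actors from saved start transforms with index-staggered, clamped progress.
; Add动画_Actor and Add动画_Comp append runtime entries to 动画队列, which Tick animates by elapsed time and removes past completion.
; The construction script can draw debug boxes around controlled actors.
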(event `self.ReceiveBeginPlay`
  (`self.保存起始位置信息`)
  (set `self.曲线时间` 0.0)
  (`self.更新控制队列`)
  (if (`self.开始即播放`)
    (`KismetSystemLibrary.Delay` (`self.开始时间`))
    (`KismetSystemLibrary.K2_SetTimerDelegate` (delegate `播放`) 0.01 true)))

(event `播放`
  (`self.更新控制队列`)
  (set `self.曲线时间` (+ (`self.曲线时间`) (* (`self.播放速度`) 0.01))))

(event `Add动画_Actor`
  (params (`播放对象` :type "Actor Object Reference") (`播放速度` :type "Float (double-precision)") (`延时开始` :type "Float (double-precision)" :default 0.0))
  ;[0 0 1] 注释
  (`KismetArrayLibrary.Array_Add` (`self.动画队列`) (make `/Game/功能实现/动画/S_动画对象` (`Actor.RootComponent` `播放对象`) (`self.GetTransform` `播放对象`) `播放速度` (`KismetSystemLibrary.GetGameTimeInSeconds`))))

(event `self.ReceiveTick`
  (params (DeltaSeconds :type "Float (single-precision)"))
  ;[0 0 1] 注释
  (`/Engine/EditorBlueprintResources/StandardMacros.CompareInt` (`KismetArrayLibrary.Array_Length` (`self.动画队列`))
    (:`>`
      (for (_array_element _array_index) (`self.动画队列`)
        (bind _returnvalue (* (`.速度速度_8_4CC7EEE94924864E37919594AEE56AF1` (break `/Game/功能实现/动画/S_动画对象` _array_element)) (- (`KismetSystemLibrary.GetGameTimeInSeconds`) (`.开始时间_7_C5CE108A45B5C93CE2A42CBEB6BEF95D` (break `/Game/功能实现/动画/S_动画对象` _array_element)))))
        (`/Engine/EditorBlueprintResources/StandardMacros.CompareFloat` _returnvalue 1.0
          (:`>`
            (`KismetArrayLibrary.Array_Remove` (`self.动画队列`) _array_index))
          (:`==`
            (`self.动画执行` (break `/Game/功能实现/动画/S_动画对象` _array_element) (`.初始变换_12_D557D55546F0122BAA589E94704262AC` (break `/Game/功能实现/动画/S_动画对象` _array_element)) _returnvalue :!label _label))
          (:`<`
            (goto _label)))))))

(event `Add动画_Comp`
  (params (`播放对象` :type "SceneComponent Object Reference") (`播放速度` :type "Float (double-precision)") (`延时开始` :type "Float (double-precision)"))
  ;[0 0 1] 注释
  (`/Engine/EditorBlueprintResources/StandardMacros.IsValid` `播放对象`
    (:`Is Valid`
      (`KismetArrayLibrary.Array_Add` (`self.动画队列`) (make `/Game/功能实现/动画/S_动画对象` `播放对象` (`SceneComponent.K2_GetComponentToWorld` `播放对象`) `播放速度` (+ `延时开始` (`KismetSystemLibrary.GetGameTimeInSeconds`)))))))

(fn `UserConstructionScript`
  (if (`self.显示被控制对象`)
    (for _array_element (`self.控制队列`)
      (bind (_origin _boxextent) (`self.GetActorBounds` _array_element false false))
      (`KismetSystemLibrary.DrawDebugBox` _origin (+ _boxextent (10.0 10.0 10.0)) (struct :`G` 1.0 :`A` 1.0) (struct) 1.0 5.0))
    (set `self.显示被控制对象` false)))

(fn `保存起始位置信息`
  (for (_array_element _array_index) (`self.控制队列`)
    (`/Engine/EditorBlueprintResources/StandardMacros.IsValid` _array_element
      (:`Is Valid`
        (bind (_returnvalue_location _returnvalue_rotation) (`KismetMathLibrary.BreakTransform` (`self.GetTransform` _array_element)))
        (`KismetArrayLibrary.Array_Set` (`self.初始变换`) _array_index (`KismetMathLibrary.MakeTransform` _returnvalue_location _returnvalue_rotation) true)
        (`self.SetActorScale3D` _array_element _returnvalue_location)))))

(fn `动画执行`
  (params (`执行对象` :type "SceneComponent Object Reference") (`初始变换` :type "Transform Structure") (`执行时间` :type "Float (double-precision)")))

(fn `更新控制队列`
  (for (_array_element _array_index) (`self.控制队列`)
    (`self.动画执行` (`Actor.RootComponent` _array_element) (`|GetArrayItem` (`self.初始变换`) _array_index) (`KismetMathLibrary.FClamp` (- (`self.曲线时间`) (* _array_index (`self.队列间隔`)))))))
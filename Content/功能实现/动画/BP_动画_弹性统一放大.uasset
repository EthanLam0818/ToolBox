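; BP_动画_弹性统一放大 is an animation Blueprint actor that scales a target object up from zero to its initial size, with an elastic effect implied by its name.
; Its 动画执行 function samples the 动画曲线 float curve at the given time to lerp scale toward the stored 初始变换.
; Each call sets the world transform, keeping initial location and rotation.
; The event graph holds only disabled default events, so timing comes from outside.
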(fn `UserConstructionScript`
  (`parent.UserConstructionScript`))

(fn `动画执行`
  (params (`执行对象` :type "SceneComponent Object Reference") (`初始变换` :type "Transform Structure") (`执行时间` :type "Float (double-precision)"))
  (`SceneComponent.K2_SetWorldTransform` `执行对象` (`KismetMathLibrary.MakeTransform` `初始变换_Location` `初始变换_Rotation` (`KismetMathLibrary.VLerp` (0.0 0.0 0.0) `初始变换_Scale` (`CurveFloat.GetFloatValue` (`self.动画曲线`) `执行时间`))) false false))
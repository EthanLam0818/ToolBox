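; BP_BaseSplineExt is a spline shape actor that derives a rounded-corner copy of its Spline at construction time.
; BuildSpline sets the source points to linear, then fills a newly added TempSpline with points interpolated along each segment by the 圆角 (corner rounding) ratio.
; Tangents follow segment direction to curve the corners: ratios below half give two points per segment, exactly half gives a single midpoint.
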(fn `BuildSpline`
  (locals (point :type "Array of Vector Structure"))
  (bind _returnvalue (`KismetMathLibrary.Conv_DoubleToVector` 2.0))
  (bind _tempspline (`self.TempSpline`))
  (bind _spline (`self.Spline`))
  (bind _spline_2 (`self.Spline`))
  (bind _spline_3 (`self.Spline`))
  (bind _tempspline_2 (`self.TempSpline`))
  (bind _tempspline_3 (`self.TempSpline`))
  (bind `_圆角` (`self.圆角`))
  (bind _returnvalue_2 (`SplineComponent.GetNumberOfSplinePoints` (`self.Spline`)))
  (bind _returnvalue_3 (`SplineComponent.IsClosedLoop` (`self.Spline`)))
  (for _index (range (`SplineComponent.GetNumberOfSplinePoints` _spline))
    (`SplineComponent.SetSplinePointType` _spline _index "Linear" true))
  (`KismetArrayLibrary.Array_Clear` (`local.point`))
  (bind _returnvalue_4 (`AddComponent|NODE_AddSplineComponent-0`))
  (bind _output_get (set `self.TempSpline` _returnvalue_4))
  (`SplineComponent.ClearSplinePoints` _output_get true)
  (if (not (`SplineComponent.IsClosedLoop` (`self.Spline`)))
    (`SplineComponent.AddSplinePoint` _tempspline_2 (`SplineComponent.GetLocationAtSplinePoint` _spline 0 "Local") "Local" true)
    (`SplineComponent.SetTangentAtSplinePoint` _tempspline_2 0 (0.0 0.0 0.0) "Local" true))
  (for _index_2 (range (+ (`KismetMathLibrary.SelectInt` _returnvalue_2 (- _returnvalue_2 2) (`SplineComponent.IsClosedLoop` (`self.Spline`))) 1))
    (bind _returnvalue_5 (`SplineComponent.GetLocationAtSplinePoint` _spline_3 _index_2 "Local"))
    (bind _returnvalue_6 (+ _index_2 1))
    (bind _returnvalue_7 (`SplineComponent.GetLocationAtSplinePoint` _spline_3 (`KismetMathLibrary.SelectInt` 0 _returnvalue_6 (> _returnvalue_6 (- (`SplineComponent.GetNumberOfSplinePoints` (`self.Spline`)) 1))) "Local"))
    (bind _returnvalue_8 (`KismetMathLibrary.VLerp` _returnvalue_5 _returnvalue_7 `_圆角`))
    (`SplineComponent.AddSplinePoint` _tempspline_3 _returnvalue_8 "Local" true)
    (`/Engine/EditorBlueprintResources/StandardMacros.CompareFloat` `_圆角` 0.5
      (:`==`
        (`SplineComponent.SetTangentAtSplinePoint` _tempspline_3 (`KismetMathLibrary.SelectInt` _index_2 _returnvalue_6 (`SplineComponent.IsClosedLoop` (`self.Spline`))) (- _returnvalue_7 _returnvalue_5) "Local" true)
        (`SplineComponent.SetTangentAtSplinePoint` _tempspline (`KismetMathLibrary.SelectInt` _index_2 _returnvalue_6 (`SplineComponent.IsClosedLoop` (`self.Spline`))) (- _returnvalue_7 _returnvalue_5) "Local" true))
      (:`<`
        (bind _returnvalue_9 (* _index_2 2))
        (bind _returnvalue_10 (+ _returnvalue_9 1))
        (`SplineComponent.SetTangentAtSplinePoint` _tempspline (`KismetMathLibrary.SelectInt` _returnvalue_9 _returnvalue_10 _returnvalue_3) (* (- _returnvalue_8 _returnvalue_5) _returnvalue) "Local" true)
        (bind _returnvalue_11 (`KismetMathLibrary.VLerp` _returnvalue_7 _returnvalue_5 `_圆角`))
        (`SplineComponent.AddSplinePoint` _tempspline _returnvalue_11 "Local" true)
        (`SplineComponent.SetTangentAtSplinePoint` _tempspline (`KismetMathLibrary.SelectInt` _returnvalue_10 (+ _returnvalue_9 2) _returnvalue_3) (* (- _returnvalue_7 _returnvalue_11) _returnvalue) "Local" true))))
  (`SplineComponent.AddSplinePoint` (`self.TempSpline`) (`SplineComponent.GetLocationAtSplinePoint` _spline_2 (- (`SplineComponent.GetNumberOfSplinePoints` _spline_2) 1) "Local") "Local" true))

(fn `UserConstructionScript`
  (`self.BuildSpline`))
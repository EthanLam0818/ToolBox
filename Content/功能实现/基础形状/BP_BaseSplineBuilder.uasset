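; BP_BaseSplineBuilder is a base actor for building shapes from mesh segments along a spline.
; Its 构建SplineMesh function takes a spline, mesh, material and color, then adds a SplineMeshComponent per 物体长度 interval, with endpoints and direction tangents sampled by distance.
; Segments get 宽度缩放 width scaling, a "color" material parameter and no shadow casting.
; The construction script and event graph are empty, so the function runs only when called.
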(fn `UserConstructionScript`)

(fn `构建SplineMesh`
  (params (Spline :type "SplineComponent Object Reference") (NewMesh :type "StaticMesh Object Reference") (Material :type "MaterialInterface Object Reference") (InLinearColor :type "LinearColor Structure"))
  (bind _returnvalue (`SplineComponent.GetSplineLength` Spline))
  (bind `_物体长度` (`self.物体长度`))
  (bind `_宽度缩放` (`self.宽度缩放`))
  (bind _returnvalue_2 (`KismetMathLibrary.FFloor` (/ _returnvalue `_物体长度`)))
  (bind _returnvalue_3 (== 0 _returnvalue_2))
  (for _index (range (+ _returnvalue_2 1))
    (bind _returnvalue_4 (`AddComponent|NODE_AddSplineMeshComponent-0`))
    (`StaticMeshComponent.SetStaticMesh` _returnvalue_4 NewMesh)
    (bind _returnvalue_5 (* `_物体长度` _index))
    (bind _returnvalue_6 (* `_物体长度` (+ _index 1)))
    (`SplineMeshComponent.SetStartAndEnd` _returnvalue_4 (`SplineComponent.GetLocationAtDistanceAlongSpline` Spline _returnvalue_5 "Local") (`SplineComponent.GetDirectionAtDistanceAlongSpline` Spline _returnvalue_5 "Local") (`KismetMathLibrary.SelectVector` (`SplineComponent.GetLocationAtDistanceAlongSpline` Spline _returnvalue "Local") (`SplineComponent.GetLocationAtDistanceAlongSpline` Spline _returnvalue_6 "Local") _returnvalue_3) (`KismetMathLibrary.SelectVector` (`SplineComponent.GetDirectionAtDistanceAlongSpline` Spline _returnvalue "Local") (`SplineComponent.GetDirectionAtDistanceAlongSpline` Spline _returnvalue_6 "Local") _returnvalue_3) true)
    (`SplineMeshComponent.SetStartAndEnd` _returnvalue_4 (`SplineComponent.GetLocationAtDistanceAlongSpline` Spline _returnvalue_5 "Local") (`SplineComponent.GetDirectionAtDistanceAlongSpline` Spline _returnvalue_5 "Local") (`KismetMathLibrary.SelectVector` (`SplineComponent.GetLocationAtDistanceAlongSpline` Spline _returnvalue "Local") (`SplineComponent.GetLocationAtDistanceAlongSpline` Spline _returnvalue_6 "Local") _returnvalue_3) (`KismetMathLibrary.SelectVector` (`SplineComponent.GetDirectionAtDistanceAlongSpline` Spline _returnvalue "Local") (`SplineComponent.GetDirectionAtDistanceAlongSpline` Spline _returnvalue_6 "Local") _returnvalue_3) true)
    (`SplineMeshComponent.SetStartScale` _returnvalue_4 (`KismetMathLibrary.MakeVector2D` `_宽度缩放` 1.0) true)
    (`SplineMeshComponent.SetStartScale` _returnvalue_4 (`KismetMathLibrary.MakeVector2D` `_宽度缩放` 1.0) true)
    (`SplineMeshComponent.SetEndScale` _returnvalue_4 (`KismetMathLibrary.MakeVector2D` `_宽度缩放` 1.0) true)
    (`PrimitiveComponent.SetMaterial` _returnvalue_4 0 Material)
    (`MeshComponent.SetVectorParameterValueOnMaterials` _returnvalue_4 "color" (`KismetMathLibrary.Conv_LinearColorToVector` InLinearColor))
    (`PrimitiveComponent.SetCastShadow` _returnvalue_4 false)))
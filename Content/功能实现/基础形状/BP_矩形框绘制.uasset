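; Rectangle-frame actor that draws a rounded-corner outline with optional fill, built in the construction script from size, corner radius and colors.
; Four corners become an eight-point spline with tangents shaping the rounded corners, which feeds spline meshes for the colored edge.
; The box extent follows the rectangle size.
; When enabled, the fill samples that spline into a procedural triangle-fan mesh, slightly lowered, with material-driven color and opacity.
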(fn `UserConstructionScript`
  (bind (`_矩形大小_x` `_矩形大小_y`) (`KismetMathLibrary.BreakVector2D` (`self.矩形大小`)))
  (`self.构建矩形spline`)
  (`self.构建SplineMesh` (`self.NewVar_0`) "/Game/StarterContent/Shapes/Shape_Plane.Shape_Plane" "/Game/功能实现/基础形状/NewMaterial.NewMaterial" (`self.边缘颜色`))
  (`BoxComponent.SetBoxExtent` (`self.Box`) (`KismetMathLibrary.MakeVector` (/ `_矩形大小_x` 2.0) (/ `_矩形大小_y` 2.0) 50.0) true)
  (if (`self.填充`)
    (`self.填充矩形mesh` "/Game/功能实现/基础形状/NewMaterial.NewMaterial" (`self.填充颜色`))))

(fn `填充矩形mesh`
  (params (Material :type "MaterialInterface Object Reference") (ParameterValue :type "LinearColor Structure" :default (struct :`R` 0.5 :`G` 0.5 :`B` 0.5 :`A` 1.0)))
  (locals (NewLocalVar_0 :type "Array of Vector Structure") (NewLocalVar_1 :type "Array of Integer") (NewLocalVar_2 :type Integer :default 10))
  (bind (_r _g _b _a) (`KismetMathLibrary.BreakColor` ParameterValue))
  (bind _newlocalvar_1 (`local.NewLocalVar_1`))
  (bind _newlocalvar_2 (`local.NewLocalVar_2`))
  (bind _newvar_0 (`self.NewVar_0`))
  (`KismetArrayLibrary.Array_Clear` (`local.NewLocalVar_0`))
  (`KismetArrayLibrary.Array_Clear` (`local.NewLocalVar_1`))
  (`KismetArrayLibrary.Array_Add` (`local.NewLocalVar_0`))
  (for _index (range 8)
    (for _index_2 (range (+ _newlocalvar_2 1))
      (`KismetArrayLibrary.Array_Add` (`local.NewLocalVar_0`) (`SplineComponent.GetLocationAtDistanceAlongSpline` (`self.NewVar_0`) (`KismetMathLibrary.Lerp` (`SplineComponent.GetDistanceAlongSplineAtSplinePoint` _newvar_0 _index) (`SplineComponent.GetDistanceAlongSplineAtSplinePoint` _newvar_0 (+ _index 1)) (/ (`KismetMathLibrary.Conv_IntToDouble` _index_2) (`KismetMathLibrary.Conv_IntToDouble` _newlocalvar_2))) "Local"))))
  (for (_ _array_index) (`local.NewLocalVar_0`)
    (bind _returnvalue (* _array_index 3))
    (`KismetArrayLibrary.Array_Set` _newlocalvar_1 _returnvalue 0 true)
    (`KismetArrayLibrary.Array_Set` _newlocalvar_1 (+ _returnvalue 1) (+ _array_index 1) true)
    (`KismetArrayLibrary.Array_Set` _newlocalvar_1 (+ _returnvalue 2) (+ _array_index 2) true))
  (bind _returnvalue_2 (`AddComponent|NODE_AddProceduralMeshComponent-2` :`RelativeTransform` (`KismetMathLibrary.MakeTransform` (0.0 0.0 -0.01))))
  (`ProceduralMeshComponent.CreateMeshSection_LinearColor` :`self` _returnvalue_2 :`Vertices` (`local.NewLocalVar_0`) :`Triangles` (`local.NewLocalVar_1`))
  (`PrimitiveComponent.SetMaterial` _returnvalue_2 0 Material)
  (`MeshComponent.SetVectorParameterValueOnMaterials` _returnvalue_2 "color" (`KismetMathLibrary.MakeVector` _r _g _b))
  (`MeshComponent.SetScalarParameterValueOnMaterials` _returnvalue_2 "opacity" _a))

(fn `构建矩形spline`
  (locals (NewLocalVar_0 :type "Array of Vector2D Structure") (NewLocalVar_3 :type "SplineComponent Object Reference"))
  (bind `_矩形大小` (`self.矩形大小`))
  (bind _newvar_0 (`self.NewVar_0`))
  (bind _array (`self.Array`))
  (bind _points (`self.Points`))
  (bind _points_2 (`self.Points`))
  (bind _returnvalue (`KismetArrayLibrary.Array_Length` _array))
  (set `self.Array` (`|MakeArray` (`KismetMathLibrary.Conv_Vector2DToVector` (* `_矩形大小` (-0.5 -0.5))) (`KismetMathLibrary.Conv_Vector2DToVector` (* `_矩形大小` (-0.5 0.5))) (`KismetMathLibrary.Conv_Vector2DToVector` (* `_矩形大小` (0.5 0.5))) (`KismetMathLibrary.Conv_Vector2DToVector` (* `_矩形大小` (0.5 -0.5)))))
  (`SplineComponent.SetSplinePoints` (`self.Spline`) (`self.Array`) "Local" true)
  (for (_ _array_index) (`self.Array`)
    (`SplineComponent.SetSplinePointType` (`self.Spline`) _array_index "Linear" true))
  (`KismetArrayLibrary.Array_Clear` _points)
  (`KismetArrayLibrary.Array_Resize` _points 8)
  (bind _returnvalue_2 (`AddComponent|NODE_AddSplineComponent-1`))
  (bind _output_get (set `self.NewVar_0` _returnvalue_2))
  (`SplineComponent.ClearSplinePoints` _output_get true)
  (`SplineComponent.SetSplinePoints` (`self.NewVar_0`) (`self.Points`) "Local" true)
  (for (_array_element _array_index_2) _array
    (bind _returnvalue_3 (* _array_index_2 2))
    (bind _returnvalue_4 (- _array_index_2 1))
    (bind _output (`|GetArrayItem` _array (`KismetMathLibrary.SelectInt` (- _returnvalue 1) _returnvalue_4 (< _returnvalue_4 0))))
    (bind _returnvalue_5 (+ _array_element (* (`KismetMathLibrary.Normal` (- _output _array_element)) (`self.圆角半径`))))
    (`KismetArrayLibrary.Array_Set` _points_2 _returnvalue_3 _returnvalue_5 true)
    (`SplineComponent.SetLocationAtSplinePoint` _newvar_0 _returnvalue_3 _returnvalue_5 "Local" true)
    (`SplineComponent.SetTangentAtSplinePoint` _newvar_0 _returnvalue_3 (* (`KismetMathLibrary.Normal` (- _array_element _output)) (* 2.0 (`self.圆角半径`))) "Local" true)
    (bind _returnvalue_6 (+ _returnvalue_3 1))
    (bind _returnvalue_7 (* (`KismetMathLibrary.Normal` (- (`|GetArrayItem` _array (mod (+ _array_index_2 1) _returnvalue)) _array_element)) (`self.圆角半径`)))
    (bind _returnvalue_8 (+ _array_element _returnvalue_7))
    (`KismetArrayLibrary.Array_Set` _points_2 _returnvalue_6 _returnvalue_8 true)
    (`SplineComponent.SetLocationAtSplinePoint` _newvar_0 _returnvalue_6 _returnvalue_8 "Local" true)
    (`SplineComponent.SetTangentAtSplinePoint` _newvar_0 _returnvalue_6 _returnvalue_7 "Local" true)))
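; Construction-time tool actor that places copies of a static mesh at regular intervals along its spline.
; The construction script calls 沿路径添加网格, which derives the count from spline length divided by spacing (间距) plus object length (物体长度).
; Each added mesh component takes only its local-space location from the spline, with no rotation following the curve.
; The event graph has no active logic.
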(fn `UserConstructionScript`
  (`self.沿路径添加网格`))

(fn `沿路径添加网格`
  (bind _returnvalue (+ (`self.间距`) (`self.物体长度`)))
  (for _index (range (+ (`KismetMathLibrary.FFloor` (/ (`SplineComponent.GetSplineLength` (`self.Spline`)) _returnvalue)) 1))
    (`AddComponent|NODE_AddStaticMeshComponent-0` :`RelativeTransform` (`KismetMathLibrary.MakeTransform` (`SplineComponent.GetLocationAtDistanceAlongSpline` (`self.Spline`) (* (`KismetMathLibrary.Conv_IntToDouble` _index) _returnvalue) "Local")))))